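; Locked door for a first-person level that the player opens once with a matching key, with a prompt widget on one side.
; An overlap trigger on the left shows or hides the prompt for the player while the door is closed.
; Interact looks up DoorName in the character's KeyList, consumes the key and swings the door open via a timeline yaw lerp.
; Without the key, it displays a fading hint dialogue widget.
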(event `self.TriggerLeft.OnComponentBeginOverlap`
  (params (OverlappedComponent :type "PrimitiveComponent Object Reference") (OtherActor :type "Actor Object Reference") (OtherComp :type "PrimitiveComponent Object Reference") (OtherBodyIndex :type Integer) (bFromSweep :type Boolean) (SweepResult :type "HitResult Structure (by ref)"))
  ;[1 1 1] Set widgets visibility related to direction u come
  (if (`self.DoorOpened?`)
    _
    (elif (`self.ActorHasTag` OtherActor "Player")
      (`SceneComponent.SetVisibility` (`self.WidgetLeft`) true false))))

(event `self.TriggerLeft.OnComponentEndOverlap`
  (params (OverlappedComponent :type "PrimitiveComponent Object Reference") (OtherActor :type "Actor Object Reference") (OtherComp :type "PrimitiveComponent Object Reference") (OtherBodyIndex :type Integer))
  ;[1 1 1] Set widgets visibility related to direction u come
  (if (`self.DoorOpened?`)
    _
    (elif (`self.ActorHasTag` OtherActor "Player")
      (`SceneComponent.SetVisibility` (`self.WidgetLeft`) false false))))

(event `self.Interact`
  (bind _doorname (`self.DoorName`))
  ;[1 1 1] Player can open door only 1 time with the check, timeline make a lerp on door rotation to reach open position
  (bind _asbp_first_person_character (cast `/Game/LostBalance/Blueprints/Player/BP_FirstPersonCharacter` (`GameplayStatics.GetPlayerCharacter` 0)))
  (bind _keylist (`/Game/LostBalance/Blueprints/Player/BP_FirstPersonCharacter.KeyList` _asbp_first_person_character))
  (if (`KismetArrayLibrary.Array_Contains` _keylist _doorname)
    (`KismetArrayLibrary.Array_RemoveItem` _keylist _doorname)
    (if (not (`self.DoorOpened?`))
      (set `self.DoorOpened?` true)
      (`SceneComponent.SetVisibility` (`self.WidgetLeft`) false false)
      (bind (_direction _dooropening) (`Timeline|DoorOpening` :!via `PlayFromStart`)
        (:`Update`
          (`SceneComponent.K2_SetRelativeRotation` (`self.DoorNoKey`) (`KismetMathLibrary.MakeRotator` 0.0 0.0 (`KismetMathLibrary.Lerp` 0.0 100.0 _dooropening)) false false))))
    (else
      (bind _returnvalue (`|CreateWidget` "/Game/LostBalance/UI/Widgets/WBP_TextDialogue.WBP_TextDialogue_C" (`GameplayStatics.GetPlayerController` 0)))
      (`/Game/LostBalance/UI/Widgets/WBP_TextDialogue.Set TextandDelayfadeout` _returnvalue (`self.DialogueHint`) (`self.DialogueFadeOutDelay`))
      (`UserWidget.AddToViewport` _returnvalue 0))))

(fn `UserConstructionScript`)