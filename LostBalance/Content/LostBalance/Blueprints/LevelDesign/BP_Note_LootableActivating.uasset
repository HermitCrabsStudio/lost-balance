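; BP_Note_LootableActivating is a collectible note pickup whose trigger overlaps can be switched on through ActivateOverlap.
; TriggerArea shows or hides its prompt widget as an actor tagged Player enters or leaves.
; Interact passes SwitchIndexNote to the first-person character's CallNoteWidget, then destroys the actor.
; It then shows a fading upper-screen message with the character's NoteCounter out of six notes found.
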(event `Activate Overlap`
  (set `PrimitiveComponent.bGenerateOverlapEvents` true (`self.Trigger Area`)))

(event `self.Trigger Area.OnComponentBeginOverlap`
  (params (OverlappedComponent :type "PrimitiveComponent Object Reference") (OtherActor :type "Actor Object Reference") (OtherComp :type "PrimitiveComponent Object Reference") (OtherBodyIndex :type Integer) (bFromSweep :type Boolean) (SweepResult :type "HitResult Structure (by ref)"))
  ;[1 1 1] Set Widget Visibility
  (if (`self.ActorHasTag` OtherActor "Player")
    (`SceneComponent.SetVisibility` (`self.Widget`) true false)))

(event `self.Trigger Area.OnComponentEndOverlap`
  (params (OverlappedComponent :type "PrimitiveComponent Object Reference") (OtherActor :type "Actor Object Reference") (OtherComp :type "PrimitiveComponent Object Reference") (OtherBodyIndex :type Integer))
  ;[1 1 1] Set Widget Visibility
  (if (`self.ActorHasTag` OtherActor "Player")
    (`SceneComponent.SetVisibility` (`self.Widget`) false false)))

(event `self.Interact`
  ;[1 1 1] Event called on object interaction
  (bind _asbp_first_person_character (cast `/Game/LostBalance/Blueprints/Player/BP_FirstPersonCharacter` (`GameplayStatics.GetPlayerCharacter` 0)))
  (`/Game/LostBalance/Blueprints/Player/BP_FirstPersonCharacter.CallNoteWidget` _asbp_first_person_character (`self.SwitchIndexNote`))
  (`self.K2_DestroyActor`)
  (`self.Call Note Counter`))

(event `Call Note Counter`
  ;[1 1 1] Call note counter
  (bind _asbp_first_person_character (cast `/Game/LostBalance/Blueprints/Player/BP_FirstPersonCharacter` (`GameplayStatics.GetPlayerCharacter` 0)))
  (bind _returnvalue (`|CreateWidget` "/Game/LostBalance/UI/Widgets/WBP_TextDialogueUpperScreen.WBP_TextDialogueUpperScreen_C" (`GameplayStatics.GetPlayerController` 0)))
  (`/Game/LostBalance/UI/Widgets/WBP_TextDialogueUpperScreen.Set TextandDelayfadeout` _returnvalue (`KismetStringLibrary.Concat_StrStr` (`KismetStringLibrary.Conv_Int64ToString` (`KismetMathLibrary.FTrunc64` (`/Game/LostBalance/Blueprints/Player/BP_FirstPersonCharacter.NoteCounter` _asbp_first_person_character))) " / 6 - NOTE FOUND") 5.0)
  (`UserWidget.AddToViewport` _returnvalue 0))

(fn `UserConstructionScript`)