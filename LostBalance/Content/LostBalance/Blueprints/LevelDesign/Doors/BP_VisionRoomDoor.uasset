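; An interactable door for vision rooms that either swings open once or acts as locked when its VisionEvent flag is set.
; Left and right triggers show the opposite-side prompt to the player and record the approach direction.
; Interact plays a random opening sound and uses timelines to rotate the door away in the matching direction.
; When locked, it plays a locked sound and, the first time only, shows a dialogue widget.
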(event `self.TriggerLeft.OnComponentBeginOverlap`
  (params (OverlappedComponent :type "PrimitiveComponent Object Reference") (OtherActor :type "Actor Object Reference") (OtherComp :type "PrimitiveComponent Object Reference") (OtherBodyIndex :type Integer) (bFromSweep :type Boolean) (SweepResult :type "HitResult Structure (by ref)"))
  ;[1 1 1] Set widgets visibility related to direction u come
  (if (not (`self.VisionEvent?`))
    (if (`self.DoorOpened?`)
      _
      (elif (`self.ActorHasTag` OtherActor "Player")
        (`SceneComponent.SetVisibility` (`self.WidgetRight`) true false)
        (set `self.Direction` false)))))

(event `self.TriggerLeft.OnComponentEndOverlap`
  (params (OverlappedComponent :type "PrimitiveComponent Object Reference") (OtherActor :type "Actor Object Reference") (OtherComp :type "PrimitiveComponent Object Reference") (OtherBodyIndex :type Integer))
  ;[1 1 1] Set widgets visibility related to direction u come
  (if (not (`self.VisionEvent?`))
    (if (`self.DoorOpened?`)
      _
      (elif (`self.ActorHasTag` OtherActor "Player")
        (`SceneComponent.SetVisibility` (`self.WidgetRight`) false false)))))

(event `self.TriggerRight.OnComponentBeginOverlap`
  (params (OverlappedComponent :type "PrimitiveComponent Object Reference") (OtherActor :type "Actor Object Reference") (OtherComp :type "PrimitiveComponent Object Reference") (OtherBodyIndex :type Integer) (bFromSweep :type Boolean) (SweepResult :type "HitResult Structure (by ref)"))
  ;[1 1 1] Set widgets visibility related to direction u come
  (if (not (`self.VisionEvent?`))
    (if (`self.DoorOpened?`)
      _
      (elif (`self.ActorHasTag` OtherActor "Player")
        (`SceneComponent.SetVisibility` (`self.WidgetLeft`) true false)
        (set `self.Direction` true)))))

(event `self.TriggerRight.OnComponentEndOverlap`
  (params (OverlappedComponent :type "PrimitiveComponent Object Reference") (OtherActor :type "Actor Object Reference") (OtherComp :type "PrimitiveComponent Object Reference") (OtherBodyIndex :type Integer))
  ;[1 1 1] Set widgets visibility related to direction u come
  (if (not (`self.VisionEvent?`))
    (if (`self.DoorOpened?`)
      _
      (elif (`self.ActorHasTag` OtherActor "Player")
        (`SceneComponent.SetVisibility` (`self.WidgetLeft`) false false)))))

(event `self.Interact`
  ;[1 1 1] Player can open door only 1 time with the check, timeline make a lerp on door rotation to reach open position
  (if (not (`self.VisionEvent?`))
    (if (not (`self.DoorOpened?`))
      (set `self.DoorOpened?` true)
      (`SceneComponent.SetVisibility` (`self.WidgetLeft`) false false)
      (`SceneComponent.SetVisibility` (`self.WidgetRight`) false false)
      (if (`self.Direction`)
        (`/Game/LostBalance/Blueprints/LevelDesign/Doors/BPC_DoorOpeningSound.Play Random Sound` (`self.BPC_DoorOpeningSound`))
        (bind (_direction _dooropening) (`Timeline|DoorOpening` :!via `PlayFromStart`)
          (:`Update`
            (`SceneComponent.K2_SetRelativeRotation` (`self.DoorNoKey`) (`KismetMathLibrary.MakeRotator` 0.0 0.0 (`KismetMathLibrary.Lerp` 0.0 (`self.OpenAnglew`) _dooropening)) false false)))
        (else
          (`/Game/LostBalance/Blueprints/LevelDesign/Doors/BPC_DoorOpeningSound.Play Random Sound` (`self.BPC_DoorOpeningSound`))
          (bind (_direction_2 _dooropening_2) (`Timeline|Timeline` :!via `PlayFromStart`)
            (:`Update`
              (`SceneComponent.K2_SetRelativeRotation` (`self.DoorNoKey`) (`KismetMathLibrary.MakeRotator` 0.0 0.0 (`KismetMathLibrary.Lerp` 0.0 (* (`self.OpenAnglew`) -1.0) _dooropening_2)) false false))))))
    (else
      (`GameplayStatics.PlaySound2D` "/Game/LostBalance/Assets/SFX/locked_door.locked_door" 1.0 1.0 0.0 null null)
      (`/Engine/EditorBlueprintResources/StandardMacros.DoOnce` false
        (:`Completed`
          (`self.Vision Event`))))))

(event `Vision Event`
  ;[1 1 1] VisionEvent
  (bind _returnvalue (`|CreateWidget` "/Game/LostBalance/UI/Widgets/WBP_TextDialogue.WBP_TextDialogue_C" (`GameplayStatics.GetPlayerController` 0)))
  (`/Game/LostBalance/UI/Widgets/WBP_TextDialogue.Set TextandDelayfadeout` _returnvalue "Jack... trust me, please" 5.0 true)
  (`UserWidget.AddToViewport` _returnvalue 0))

(fn `UserConstructionScript`)