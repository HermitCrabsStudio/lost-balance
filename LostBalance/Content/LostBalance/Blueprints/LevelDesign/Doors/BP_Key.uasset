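; BP_Key is a key pickup that the player loots through interaction.
; A sphere overlap shows its widget while an actor tagged Player is inside and hides it on exit.
; The Interact event passes KeyName to LootKey on BP_FirstPersonCharacter, then destroys the key actor.
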(event `self.Sphere.OnComponentBeginOverlap`
  (params (OverlappedComponent :type "PrimitiveComponent Object Reference") (OtherActor :type "Actor Object Reference") (OtherComp :type "PrimitiveComponent Object Reference") (OtherBodyIndex :type Integer) (bFromSweep :type Boolean) (SweepResult :type "HitResult Structure (by ref)"))
  ;[1 1 1] Set widget visibility on overlap
  (if (`self.ActorHasTag` OtherActor "Player")
    (`SceneComponent.SetVisibility` (`self.Widget`) true false)))

(event `self.Sphere.OnComponentEndOverlap`
  (params (OverlappedComponent :type "PrimitiveComponent Object Reference") (OtherActor :type "Actor Object Reference") (OtherComp :type "PrimitiveComponent Object Reference") (OtherBodyIndex :type Integer))
  ;[1 1 1] Set widget visibility on overlap
  (if (`self.ActorHasTag` OtherActor "Player")
    (`SceneComponent.SetVisibility` (`self.Widget`) false false)))

(event `/Game/LostBalance/Blueprints/Technical/BPI_Interaction.Interact`
  ;[1 1 1] On interact cast the name of the key to the player and destroy
  (bind _asbp_first_person_character (cast `/Game/LostBalance/Blueprints/Player/BP_FirstPersonCharacter` (`GameplayStatics.GetPlayerCharacter` 0)))
  (`/Game/LostBalance/Blueprints/Player/BP_FirstPersonCharacter.LootKey` _asbp_first_person_character (`self.KeyName`))
  (`self.K2_DestroyActor`))

(fn `UserConstructionScript`)