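; BP_KeyActivation is a key pickup that gives its named key to the player when interacted with.
; ActivateOverlap turns on the trigger's overlap events, and the trigger shows or hides a widget as an actor tagged Player enters or leaves.
; Interact passes KeyName to BP_FirstPersonCharacter's LootKey, displays a fading "KEY OBTAINED" message on screen, then destroys the actor.
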(event `Activate Overlap`
  (set `PrimitiveComponent.bGenerateOverlapEvents` true (`self.Trigger`)))

(event `self.Trigger.OnComponentBeginOverlap`
  (params (OverlappedComponent :type "PrimitiveComponent Object Reference") (OtherActor :type "Actor Object Reference") (OtherComp :type "PrimitiveComponent Object Reference") (OtherBodyIndex :type Integer) (bFromSweep :type Boolean) (SweepResult :type "HitResult Structure (by ref)"))
  ;[1 1 1] Set widget visibility on overlap
  (if (`self.ActorHasTag` OtherActor "Player")
    (`SceneComponent.SetVisibility` (`self.Widget`) true false)))

(event `self.Trigger.OnComponentEndOverlap`
  (params (OverlappedComponent :type "PrimitiveComponent Object Reference") (OtherActor :type "Actor Object Reference") (OtherComp :type "PrimitiveComponent Object Reference") (OtherBodyIndex :type Integer))
  ;[1 1 1] Set widget visibility on overlap
  (if (`self.ActorHasTag` OtherActor "Player")
    (`SceneComponent.SetVisibility` (`self.Widget`) false false)))

(event `self.Interact`
  ;[1 1 1] On interact cast the name of the key to the player and destroy
  (bind _asbp_first_person_character (cast `/Game/LostBalance/Blueprints/Player/BP_FirstPersonCharacter` (`GameplayStatics.GetPlayerCharacter` 0)))
  (`/Game/LostBalance/Blueprints/Player/BP_FirstPersonCharacter.LootKey` _asbp_first_person_character (`self.KeyName`))
  (bind _returnvalue (`|CreateWidget` "/Game/LostBalance/UI/Widgets/WBP_TextDialogueUpperScreen.WBP_TextDialogueUpperScreen_C" (`GameplayStatics.GetPlayerController` 0)))
  (`/Game/LostBalance/UI/Widgets/WBP_TextDialogueUpperScreen.Set TextandDelayfadeout` _returnvalue "KEY OBTAINED" 3.0)
  (`UserWidget.AddToViewport` _returnvalue 0)
  (`self.K2_DestroyActor`))

(fn `UserConstructionScript`)