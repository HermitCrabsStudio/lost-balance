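; BP_Vision1_2axes is a level trigger that unlocks a vision when the player stands inside with the requested values on two emotion bars.
; At BeginPlay, each requested value's sign selects a less-or-equal or greater-or-equal comparison.
; While the player overlaps, Tick latches each met condition without resetting it.
; When both hold, it spawns BP_Enemy above itself, calls the character's VisionInteractionEvent and destroys itself.
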(event `self.ReceiveBeginPlay`
  ;[1 1 1] On start based on selected value set index for emotions bar to 0 or 1 to change the check from greater to less
  (if (< (`self.RequestValueBarLower`) 0.0)
    (set `self.SwitchIndexBarLower` 0)
    (else
      (set `self.SwitchIndexBarLower` 1)))
  (if (< (`self.RequestValueBarUpper`) 0.0)
    (set `self.SwitchIndexBarUpper` 0)
    (else
      (set `self.SwitchIndexBarUpper` 1)))
  ;[1 1 1] DEBUG
  (`KismetSystemLibrary.PrintString` (`KismetStringLibrary.Conv_IntToString` (`self.SwitchIndexBarLower`)))
  (`KismetSystemLibrary.PrintString` (`KismetStringLibrary.Conv_IntToString` (`self.SwitchIndexBarUpper`))))

(event `self.ReceiveTick`
  (params (DeltaSeconds :type "Float (single-precision)"))
  (bind _returnvalue (`self.GetTransform`))
  (bind _requestvaluebarlower (`self.RequestValueBarLower`))
  (bind _requestvaluebarupper (`self.RequestValueBarUpper`))
  ;[1 1 1] If player in area, check for the emotions values on bar 1 and 2. If values respect the AND BOOL return true and unlock vision, otherwise return false. Switch based on greater or less requested value.
  (if (`self.Player In Area?`)
    (bind _asbp_first_person_character (cast `/Game/LostBalance/Blueprints/Player/BP_FirstPersonCharacter` (`GameplayStatics.GetPlayerCharacter` 0)))
    (switch `int` (`self.SwitchIndexBarLower`)
      (:`0`
        (bind _emozione_1_copia (`/Game/LostBalance/Blueprints/Player/BP_FirstPersonCharacter.Emozione 1 Copia` _asbp_first_person_character))
        (if (<= _emozione_1_copia _requestvaluebarlower)
          (set `self.Condition1Achieved` true)))
      (:`1`
        (if (>= _emozione_1_copia _requestvaluebarlower)
          (set `self.Condition1Achieved` true))))
    (switch `int` (`self.SwitchIndexBarUpper`)
      (:`0`
        (bind _emozione_2_copia (`/Game/LostBalance/Blueprints/Player/BP_FirstPersonCharacter.Emozione 2 Copia` _asbp_first_person_character))
        (if (<= _emozione_2_copia _requestvaluebarupper)
          (set `self.Condition2Achieved` true)))
      (:`1`
        (if (>= _emozione_2_copia _requestvaluebarupper)
          (set `self.Condition2Achieved` true))))
    (if (and (`self.Condition1Achieved`) (`self.Condition2Achieved`))
      (`KismetSystemLibrary.PrintString` "VISION UNLOCKED" true true (struct :`G` 1.0 :`B` 0.007477 :`A` 1.0) 3.0)
      (`|SpawnActorFromClass` "/Game/ThirdPerson/Blueprints/BP_Enemy.BP_Enemy_C" (`KismetMathLibrary.MakeTransform` (`KismetMathLibrary.MakeVector` (.x (.location _returnvalue)) (.y (.location _returnvalue)) (+ (.z (.location _returnvalue)) 80.0)) (struct :`Yaw` 90.0)) "AdjustIfPossibleButAlwaysSpawn" "MultiplyWithRoot" null null)
      (bind _asbp_first_person_character_2 (cast `/Game/LostBalance/Blueprints/Player/BP_FirstPersonCharacter` (`GameplayStatics.GetPlayerCharacter` 0)))
      (`/Game/LostBalance/Blueprints/Player/BP_FirstPersonCharacter.VisionInteractionEvent` _asbp_first_person_character_2)
      (`self.K2_DestroyActor`)
      (else
        (`KismetSystemLibrary.PrintString` "WRONG EMOTIONS" true true (struct :`R` 1.0 :`B` 0.029075 :`A` 1.0) 3.0)))))

(event `self.TriggerArea.OnComponentBeginOverlap`
  (params (OverlappedComponent :type "PrimitiveComponent Object Reference") (OtherActor :type "Actor Object Reference") (OtherComp :type "PrimitiveComponent Object Reference") (OtherBodyIndex :type Integer) (bFromSweep :type Boolean) (SweepResult :type "HitResult Structure (by ref)"))
  ;[1 1 1] Player in Area check, using trigger area
  (if (`self.ActorHasTag` OtherActor "Player")
    (set `self.Player In Area?` true)
    (`self.SetActorTickEnabled` true)))

(event `self.TriggerArea.OnComponentEndOverlap`
  (params (OverlappedComponent :type "PrimitiveComponent Object Reference") (OtherActor :type "Actor Object Reference") (OtherComp :type "PrimitiveComponent Object Reference") (OtherBodyIndex :type Integer))
  ;[1 1 1] Player in Area check, using trigger area
  (if (`self.ActorHasTag` OtherActor "Player")
    (set `self.Player In Area?` false)))

(fn `UserConstructionScript`)