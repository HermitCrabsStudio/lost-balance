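; BP_StairSpawner is an interactable hatch that reveals a climbable ladder.
; An upper trigger shows a prompt widget, and the player's Interact call runs ActivateStairs, enabling the ladder and climbing trigger.
; A timeline swings the hatch pivot open while disabling the prompt and activation trigger.
; Entering the climbing trigger calls ActiveRayCast on the player's climbing component unless already climbing.
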(event `Activate Stairs`
  (bind _ladder (`self.Ladder`))
  ;[1 1 1] Activate stairs when called (set parameters for collision and visilibity)
  (`SceneComponent.SetVisibility` _ladder true false)
  (`PrimitiveComponent.SetCollisionEnabled` _ladder "QueryAndPhysics")
  (set `PrimitiveComponent.bGenerateOverlapEvents` true (`self.ClimbingTrigger`))
  (bind (_direction _open) (`Timeline|OpenLadder` :!via `PlayFromStart`)
    (:`Update`
      (`SceneComponent.K2_SetRelativeRotation` (`self.PivotBotola`) (`KismetMathLibrary.MakeRotator` (`KismetMathLibrary.Lerp` 0.0 110.0 _open)) false false)
      (`SceneComponent.SetVisibility` (`self.Widget`) false false)
      (set `PrimitiveComponent.bGenerateOverlapEvents` false (`self.ActivateStairsTrigger`)))))

(event `/Game/LostBalance/Blueprints/Technical/BPI_Interaction.Interact`
  ;[1 1 1] Activate stairs when called (set parameters for collision and visilibity)
  ;;[1 1 1] Interaction event (called from player, when overlap the upper volume
  (`self.Activate Stairs`))

(event `self.ClimbingTrigger.OnComponentBeginOverlap`
  (params (OverlappedComponent :type "PrimitiveComponent Object Reference") (OtherActor :type "Actor Object Reference") (OtherComp :type "PrimitiveComponent Object Reference") (OtherBodyIndex :type Integer) (bFromSweep :type Boolean) (SweepResult :type "HitResult Structure (by ref)"))
  ;[1 1 1] On overlap Set climbing to true and call active raycast from player BPC component
  (if (`self.ActorHasTag` OtherActor "Player")
    (bind _asbp_first_person_character (cast `/Game/LostBalance/Blueprints/Player/BP_FirstPersonCharacter` (`GameplayStatics.GetPlayerCharacter` 0)))
    (if (not (`/Game/LostBalance/Blueprints/Player/BP_FirstPersonCharacter.IsClimbing?` _asbp_first_person_character))
      (`/Game/LostBalance/Blueprints/Player/PlayerComponents/BPC_ClimbingComponent.Active RayCast` (`/Game/LostBalance/Blueprints/Player/BP_FirstPersonCharacter.BPC_ClimbingComponent` _asbp_first_person_character))
      (else
        (`KismetSystemLibrary.PrintString` "CALL FALSE" true true (struct :`G` 1.0 :`B` 0.064783 :`A` 1.0) 5.0)))))

(event `self.ActivateStairsTrigger.OnComponentBeginOverlap`
  (params (OverlappedComponent :type "PrimitiveComponent Object Reference") (OtherActor :type "Actor Object Reference") (OtherComp :type "PrimitiveComponent Object Reference") (OtherBodyIndex :type Integer) (bFromSweep :type Boolean) (SweepResult :type "HitResult Structure (by ref)"))
  ;[1 1 1] Toggle widget visibility
  (if (`self.ActorHasTag` OtherActor "Player")
    (`SceneComponent.SetVisibility` (`self.Widget`) true false)))

(event `self.ActivateStairsTrigger.OnComponentEndOverlap`
  (params (OverlappedComponent :type "PrimitiveComponent Object Reference") (OtherActor :type "Actor Object Reference") (OtherComp :type "PrimitiveComponent Object Reference") (OtherBodyIndex :type Integer))
  ;[1 1 1] Toggle widget visibility
  (if (`self.ActorHasTag` OtherActor "Player")
    (`SceneComponent.SetVisibility` (`self.Widget`) false false)))

(fn `UserConstructionScript`)