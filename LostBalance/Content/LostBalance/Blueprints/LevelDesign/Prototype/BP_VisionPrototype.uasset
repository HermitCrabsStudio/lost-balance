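; Prototype vision trigger that unlocks when the player's two emotion values meet requested thresholds inside its area.
; The sign of each threshold picks a less-or-equal or greater-or-equal check on Tick, and met conditions stay latched.
; Success spawns BP_Enemy, plays the player's vision effect, grants an immunity and destroys the trigger.
; First entry can show an on-screen hint; a separate event ramps up a point light.
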(event `self.ReceiveBeginPlay`
  ;[1 1 1] On start based on selected value set index for emotions bar to 0 or 1 to change the check from greater to less
  (if (< (`self.RequestValueBarLower`) 0.0)
    (set `self.SwitchIndexBarLower` 0)
    (else
      (set `self.SwitchIndexBarLower` 1)))
  (if (< (`self.RequestValueBarUpper`) 0.0)
    (set `self.SwitchIndexBarUpper` 0)
    (else
      (set `self.SwitchIndexBarUpper` 1))))

(event `self.ReceiveTick`
  (params (DeltaSeconds :type "Float (single-precision)"))
  (bind _requestvaluebarlower (`self.RequestValueBarLower`))
  (bind _requestvaluebarupper (`self.RequestValueBarUpper`))
  ;[1 1 1] If player in area, check for the emotions values on bar 1 and 2. If values respect the AND BOOL return true and unlock vision, otherwise return false. Switch based on greater or less requested value.
  (if (`self.Player In Area?`)
    (bind _asbp_first_person_character (cast `/Game/LostBalance/Blueprints/Player/BP_FirstPersonCharacter` (`GameplayStatics.GetPlayerCharacter` 0)))
    (switch `int` (`self.SwitchIndexBarLower`)
      (:`0`
        (bind _emozione_1_copia (`/Game/LostBalance/Blueprints/Player/BP_FirstPersonCharacter.Emozione 1 Copia` _asbp_first_person_character))
        (if (<= _emozione_1_copia _requestvaluebarlower)
          (set `self.Condition1Achieved` true)))
      (:`1`
        (if (>= _emozione_1_copia _requestvaluebarlower)
          (set `self.Condition1Achieved` true))))
    (switch `int` (`self.SwitchIndexBarUpper`)
      (:`0`
        (bind _emozione_2_copia (`/Game/LostBalance/Blueprints/Player/BP_FirstPersonCharacter.Emozione 2 Copia` _asbp_first_person_character))
        (if (<= _emozione_2_copia _requestvaluebarupper)
          (set `self.Condition2Achieved` true)))
      (:`1`
        (if (>= _emozione_2_copia _requestvaluebarupper)
          (set `self.Condition2Achieved` true))))
    (if (and (`self.Condition1Achieved`) (`self.Condition2Achieved`))
      (`|SpawnActorFromClass` "/Game/ThirdPerson/Blueprints/BP_Enemy.BP_Enemy_C" (`KismetMathLibrary.MakeTransform` (`SceneComponent.K2_GetComponentLocation` (`self.SpawnReferenceSagoma`)) (struct :`Yaw` 90.0)) "AdjustIfPossibleButAlwaysSpawn" "MultiplyWithRoot" null null)
      (bind _asbp_first_person_character_2 (cast `/Game/LostBalance/Blueprints/Player/BP_FirstPersonCharacter` (`GameplayStatics.GetPlayerCharacter` 0)))
      (`/Game/LostBalance/Blueprints/Player/BP_FirstPersonCharacter.VisionBasicEffect` _asbp_first_person_character_2)
      (set `/Game/LostBalance/Blueprints/Player/PlayerComponents/BPC_Immunities.Immunita2-` true (`/Game/LostBalance/Blueprints/Player/BP_FirstPersonCharacter.BPC_Immunities` _asbp_first_person_character_2))
      (`self.K2_DestroyActor`))))

(event `self.TriggerArea.OnComponentBeginOverlap`
  (params (OverlappedComponent :type "PrimitiveComponent Object Reference") (OtherActor :type "Actor Object Reference") (OtherComp :type "PrimitiveComponent Object Reference") (OtherBodyIndex :type Integer) (bFromSweep :type Boolean) (SweepResult :type "HitResult Structure (by ref)"))
  ;[1 1 1] Player in Area check, using trigger area
  (if (`self.ActorHasTag` OtherActor "Player")
    (set `self.Player In Area?` true)
    (`self.SetActorTickEnabled` true)
    (`/Engine/EditorBlueprintResources/StandardMacros.DoOnce` false
      (:`Completed`
        (if (not (`self.NoHint`))
          (bind _returnvalue (`|CreateWidget` "/Game/LostBalance/UI/Widgets/WBP_TextDialogueUpperScreen.WBP_TextDialogueUpperScreen_C" (`GameplayStatics.GetPlayerController` 0)))
          (`/Game/LostBalance/UI/Widgets/WBP_TextDialogueUpperScreen.Set TextandDelayfadeout` _returnvalue "ALIGN YOUR EMOTIONS TO INTERACT WITH THE VISION" (`self.Delay Fade Out HINT`) false)
          (`UserWidget.AddToViewport` _returnvalue 0))))))

(event `self.TriggerArea.OnComponentEndOverlap`
  (params (OverlappedComponent :type "PrimitiveComponent Object Reference") (OtherActor :type "Actor Object Reference") (OtherComp :type "PrimitiveComponent Object Reference") (OtherBodyIndex :type Integer))
  ;[1 1 1] Player in Area check, using trigger area
  (if (`self.ActorHasTag` OtherActor "Player")
    (set `self.Player In Area?` false)))

(event `Light trigger`
  (bind (_direction _light) (`Timeline|Timeline` :!via `PlayFromStart`)
    (:`Update`
      (`LightComponent.SetIntensity` (`self.PointLight`) (`KismetMathLibrary.Lerp` 0.0 75000.0 _light)))))

(fn `UserConstructionScript`)