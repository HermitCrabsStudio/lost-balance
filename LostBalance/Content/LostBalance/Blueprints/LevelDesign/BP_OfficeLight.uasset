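; BP_OfficeLight is a level-design light switch that toggles a pair of spot lights when interacted with.
; A trigger volume shows a widget component while a player-tagged actor overlaps it and hides it on exit.
; The Interact event uses a FlipFlop to switch both lights, flip the lever's rotation and play a switch sound with slight random pitch variation.
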(event `self.Trigger.OnComponentBeginOverlap`
  (params (OverlappedComponent :type "PrimitiveComponent Object Reference") (OtherActor :type "Actor Object Reference") (OtherComp :type "PrimitiveComponent Object Reference") (OtherBodyIndex :type Integer) (bFromSweep :type Boolean) (SweepResult :type "HitResult Structure (by ref)"))
  (if (`self.ActorHasTag` OtherActor "Player")
    (`SceneComponent.SetVisibility` (`self.Widget`) true false)))

(event `self.Trigger.OnComponentEndOverlap`
  (params (OverlappedComponent :type "PrimitiveComponent Object Reference") (OtherActor :type "Actor Object Reference") (OtherComp :type "PrimitiveComponent Object Reference") (OtherBodyIndex :type Integer))
  (if (`self.ActorHasTag` OtherActor "Player")
    (`SceneComponent.SetVisibility` (`self.Widget`) false false)))

(event `/Game/LostBalance/Blueprints/Technical/BPI_Interaction.Interact`
  (`/Engine/EditorBlueprintResources/StandardMacros.FlipFlop`
    (:`A`
      (`SceneComponent.SetVisibility` (`self.SpotLight`) true false)
      (`SceneComponent.SetVisibility` (`self.SpotLight1`) true false)
      (`GameplayStatics.PlaySound2D` "/Game/LostBalance/Assets/SFX/light-switch.light-switch" 1.0 (`KismetMathLibrary.RandomFloatInRange` 0.9 1.1) 0.0 null null)
      (`SceneComponent.K2_SetRelativeRotation` (`self.Lever`) (struct :`Roll` -80.0) false false))
    (:`B`
      (`SceneComponent.SetVisibility` (`self.SpotLight`) false false)
      (`SceneComponent.SetVisibility` (`self.SpotLight1`) false false)
      (`GameplayStatics.PlaySound2D` "/Game/LostBalance/Assets/SFX/light-switch.light-switch" 1.0 (`KismetMathLibrary.RandomFloatInRange` 0.9 1.1) 0.0 null null)
      (`SceneComponent.K2_SetRelativeRotation` (`self.Lever`) (struct :`Roll` 80.0) false false))))

(fn `UserConstructionScript`)