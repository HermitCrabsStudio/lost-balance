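; BP_Armadio is an interactable cabinet whose two doors swing open once and stay open.
; While it is closed, its trigger shows a prompt widget when an actor tagged Player overlaps and hides it on exit.
; Interact latches IsOpen, hides the widget, plays a 2D opening sound and runs two timelines that lerp each door's yaw to its own opening angle.
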(event `self.Trigger.OnComponentBeginOverlap`
  (params (OverlappedComponent :type "PrimitiveComponent Object Reference") (OtherActor :type "Actor Object Reference") (OtherComp :type "PrimitiveComponent Object Reference") (OtherBodyIndex :type Integer) (bFromSweep :type Boolean) (SweepResult :type "HitResult Structure (by ref)"))
  (if (`self.isOpen`)
    _
    (elif (`self.ActorHasTag` OtherActor "Player")
      (`SceneComponent.SetVisibility` (`self.Widget`) true false))))

(event `self.Trigger.OnComponentEndOverlap`
  (params (OverlappedComponent :type "PrimitiveComponent Object Reference") (OtherActor :type "Actor Object Reference") (OtherComp :type "PrimitiveComponent Object Reference") (OtherBodyIndex :type Integer))
  (if (`self.isOpen`)
    _
    (elif (`self.ActorHasTag` OtherActor "Player")
      (`SceneComponent.SetVisibility` (`self.Widget`) false false))))

(event `/Game/LostBalance/Blueprints/Technical/BPI_Interaction.Interact`
  (if (not (`self.isOpen`))
    (set `self.isOpen` true)
    (`|ExecutionSequence`
      (:`then_0`
        (bind (_direction _dooropening) (`Timeline|Timeline` :!via `PlayFromStart`)
          (:`Update`
            (`SceneComponent.K2_SetRelativeRotation` (`self.rightLocketDoor`) (`KismetMathLibrary.MakeRotator` 0.0 0.0 (`KismetMathLibrary.Lerp` 90.0 (`self.Opening Angle Right`) _dooropening)) false false))))
      (:`then_1`
        (bind (_direction_2 _dooropening_2) (`Timeline|Timeline_0` :!via `PlayFromStart`)
          (:`Update`
            (`SceneComponent.K2_SetRelativeRotation` (`self.leftLocketDoor`) (`KismetMathLibrary.MakeRotator` 0.0 0.0 (`KismetMathLibrary.Lerp` 90.0 (`self.Opening Angle Left`) _dooropening_2)) false false))))
      (:`then_2`
        (`SceneComponent.SetVisibility` (`self.Widget`) false false))
      (:`then_3`
        (`GameplayStatics.PlaySound2D` (`self.openingSound`) 0.5 0.7 0.3 null null)))))

(fn `UserConstructionScript`)