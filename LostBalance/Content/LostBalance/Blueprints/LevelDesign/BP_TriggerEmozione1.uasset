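; Level trigger volume that inflicts emotional damage on the first-person player while they stay inside it.
; Its Tick, throttled to a configurable interval, subtracts DamageEmotivo from the player's Emozione1Copia and flags EmotionalDamageActive.
; Entering enables the trigger's tick and disables the player's.
; Exiting starts the player's emotional restore delay and resets restore state, and the next tick clears the damage flag and switches itself off.
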(event `self.ReceiveBeginPlay`
  (`self.SetActorTickInterval` (`self.Tick Interval Value`)))

(event `self.ReceiveTick`
  (params (DeltaSeconds :type "Float (single-precision)"))
  ;[1 1 1] Tick any x seconds (1 actually) and cause emotional damage to BP_FirstPersonCharacter, CHECK BOOLEAN, Set emotionaldamageactive bool in player, deactive tick to optimize when not needed
  (if (`self.PlayerInArea?`)
    (bind _asbp_first_person_character (cast `/Game/LostBalance/Blueprints/Player/BP_FirstPersonCharacter` (`GameplayStatics.GetPlayerCharacter` 0)))
    (set `/Game/LostBalance/Blueprints/Player/BP_FirstPersonCharacter.Emozione 1 Copia` (- (`/Game/LostBalance/Blueprints/Player/BP_FirstPersonCharacter.Emozione 1 Copia` _asbp_first_person_character) (`self.DamageEmotivo`)) _asbp_first_person_character)
    (set `/Game/LostBalance/Blueprints/Player/BP_FirstPersonCharacter.EmotionalDamageActive?` true _asbp_first_person_character)
    (else
      (bind _asbp_first_person_character_2 (cast `/Game/LostBalance/Blueprints/Player/BP_FirstPersonCharacter` (`GameplayStatics.GetPlayerCharacter` 0)))
      (bind _output_get (set `/Game/LostBalance/Blueprints/Player/BP_FirstPersonCharacter.EmotionalDamageActive?` false _asbp_first_person_character_2))
      (`self.SetActorTickEnabled` false)
      (`KismetSystemLibrary.PrintString` (`KismetStringLibrary.Conv_BoolToString` _output_get)))))

(event `self.TriggerEmozione.OnComponentBeginOverlap`
  (params (OverlappedComponent :type "PrimitiveComponent Object Reference") (OtherActor :type "Actor Object Reference") (OtherComp :type "PrimitiveComponent Object Reference") (OtherBodyIndex :type Integer) (bFromSweep :type Boolean) (SweepResult :type "HitResult Structure (by ref)"))
  ;[1 1 1] Set Boolean on overlap and END overlap, active tick only on overlap to optimize
  (if (`self.ActorHasTag` OtherActor "Player")
    (set `self.PlayerInArea?` true)
    (`self.SetActorTickEnabled` true)
    (bind _asbp_first_person_character (cast `/Game/LostBalance/Blueprints/Player/BP_FirstPersonCharacter` (`GameplayStatics.GetPlayerCharacter` 0)))
    (`self.SetActorTickEnabled` _asbp_first_person_character false)))

(event `self.TriggerEmozione.OnComponentEndOverlap`
  (params (OverlappedComponent :type "PrimitiveComponent Object Reference") (OtherActor :type "Actor Object Reference") (OtherComp :type "PrimitiveComponent Object Reference") (OtherBodyIndex :type Integer))
  ;[1 1 1] Set Boolean on overlap and END overlap, active tick only on overlap to optimize
  (if (`self.ActorHasTag` OtherActor "Player")
    (set `self.PlayerInArea?` false)
    (bind _asbp_first_person_character (cast `/Game/LostBalance/Blueprints/Player/BP_FirstPersonCharacter` (`GameplayStatics.GetPlayerCharacter` 0)))
    (`/Game/LostBalance/Blueprints/Player/BP_FirstPersonCharacter.Set Emotional Restore Delay` _asbp_first_person_character)
    (`KismetSystemLibrary.PrintString` "TEST")
    (set `/Game/LostBalance/Blueprints/Player/BP_FirstPersonCharacter.TickRestored?` false _asbp_first_person_character)
    (set `/Game/LostBalance/Blueprints/Player/BP_FirstPersonCharacter.SwitchToRestoreIndex` 0 _asbp_first_person_character)))

(fn `UserConstructionScript`)