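; Trigger volume that applies periodic emotional damage to BP_FirstPersonCharacter while the player stands inside it.
; A string switch picks which of the two emotion values is raised or lowered and colors the game-hidden box to match.
; Overlap pauses that emotion bar's delay on enter and restarts it on exit.
; Tick runs at a set interval, is enabled on entry, and disables itself once the player has left.
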(event `Area Color visibility ON`
  ;[1 1 1] Toggle internal area color visibility (FOR EMODEX FUNCTION) 9maybe not used)
)

(event `Hide Camera Color OFF`
  ;[1 1 1] Toggle internal area color visibility (FOR EMODEX FUNCTION) 9maybe not used)
)

(event `self.ReceiveBeginPlay`
  (bind _colorbox (`self.ColorBox`))
  ;[1 1 1] Set tick interval on start
  (`self.SetActorTickInterval` (`self.Tick Interval Value`))
  ;[1 1 1] Set the color of the box at the start of the game
  (switch `string` (`self.Pick Damage Index (1+,1-,2+,2-)`)
    (:`1+`
      (`PrimitiveComponent.SetMaterial` _colorbox 0 "/Game/LostBalance/Materials/M_Blu.M_Blu"))
    (:`1-`
      (`PrimitiveComponent.SetMaterial` _colorbox 0 "/Game/LostBalance/Materials/M_Verde.M_Verde"))
    (:`2+`
      (`PrimitiveComponent.SetMaterial` _colorbox 0 "/Game/LostBalance/Materials/M_Giallo.M_Giallo"))
    (:`2-`
      (`PrimitiveComponent.SetMaterial` _colorbox 0 "/Game/LostBalance/Materials/M_Rosso.M_Rosso")))
  (`SceneComponent.SetHiddenInGame` _colorbox true false)
  (`SceneComponent.SetVisibility` _colorbox true false))

(event `self.ReceiveTick`
  (params (DeltaSeconds :type "Float (single-precision)"))
  ;[1 1 1] Tick any x seconds (1 actually) and cause emotional damage to BP_FirstPersonCharacter, CHECK BOOLEAN, Set emotionaldamageactive bool in player, deactive tick to optimize when not needed
  (if (`self.Player in Area`)
    ;;[1 1 1] Change the type of damage based on switch index (string)
    (switch `string` (`self.Pick Damage Index (1+,1-,2+,2-)`)
      (:`1+`
        (bind _asbp_first_person_character (cast `/Game/LostBalance/Blueprints/Player/BP_FirstPersonCharacter` (`GameplayStatics.GetPlayerCharacter` 0)))
        (set `/Game/LostBalance/Blueprints/Player/BP_FirstPersonCharacter.Emozione 1 Copia` (+ (`/Game/LostBalance/Blueprints/Player/BP_FirstPersonCharacter.Emozione 1 Copia` _asbp_first_person_character) (`self.DamageEmotivo`)) _asbp_first_person_character))
      (:`1-`
        (bind _asbp_first_person_character_2 (cast `/Game/LostBalance/Blueprints/Player/BP_FirstPersonCharacter` (`GameplayStatics.GetPlayerCharacter` 0)))
        (set `/Game/LostBalance/Blueprints/Player/BP_FirstPersonCharacter.Emozione 1 Copia` (- (`/Game/LostBalance/Blueprints/Player/BP_FirstPersonCharacter.Emozione 1 Copia` _asbp_first_person_character_2) (`self.DamageEmotivo`)) _asbp_first_person_character_2))
      (:`2+`
        (bind _asbp_first_person_character_3 (cast `/Game/LostBalance/Blueprints/Player/BP_FirstPersonCharacter` (`GameplayStatics.GetPlayerCharacter` 0)))
        (set `/Game/LostBalance/Blueprints/Player/BP_FirstPersonCharacter.Emozione 2 Copia` (+ (`/Game/LostBalance/Blueprints/Player/BP_FirstPersonCharacter.Emozione 2 Copia` _asbp_first_person_character_3) (`self.DamageEmotivo`)) _asbp_first_person_character_3))
      (:`2-`
        (bind _asbp_first_person_character_4 (cast `/Game/LostBalance/Blueprints/Player/BP_FirstPersonCharacter` (`GameplayStatics.GetPlayerCharacter` 0)))
        (set `/Game/LostBalance/Blueprints/Player/BP_FirstPersonCharacter.Emozione 2 Copia` (- (`/Game/LostBalance/Blueprints/Player/BP_FirstPersonCharacter.Emozione 2 Copia` _asbp_first_person_character_4) (`self.DamageEmotivo`)) _asbp_first_person_character_4)))
    (else
      (`self.SetActorTickEnabled` false))))

(event `self.TriggerArea.OnComponentBeginOverlap`
  (params (OverlappedComponent :type "PrimitiveComponent Object Reference") (OtherActor :type "Actor Object Reference") (OtherComp :type "PrimitiveComponent Object Reference") (OtherBodyIndex :type Integer) (bFromSweep :type Boolean) (SweepResult :type "HitResult Structure (by ref)"))
  (bind _returnvalue (`GameplayStatics.GetPlayerCharacter` 0))
  ;[1 1 1] Set Boolean on overlap and END overlap, active tick only on overlap to optimize
  (if (`self.ActorHasTag` OtherActor "Player")
    (set `self.Player in Area` true)
    (`self.SetActorTickEnabled` true)
    (switch `string` (`self.Pick Damage Index (1+,1-,2+,2-)`)
      (:`1+`
        (bind _asbp_first_person_character (cast `/Game/LostBalance/Blueprints/Player/BP_FirstPersonCharacter` _returnvalue :!label _label))
        (`/Game/LostBalance/Blueprints/Player/BP_FirstPersonCharacter.Stop Delay Bar 1` _asbp_first_person_character))
      (:`1-`
        (goto _label))
      (:`2+`
        (bind _asbp_first_person_character_2 (cast `/Game/LostBalance/Blueprints/Player/BP_FirstPersonCharacter` _returnvalue :!label _label_2))
        (`/Game/LostBalance/Blueprints/Player/BP_FirstPersonCharacter.Stop Delay Bar 2` _asbp_first_person_character_2))
      (:`2-`
        (goto _label_2)))))

(event `self.TriggerArea.OnComponentEndOverlap`
  (params (OverlappedComponent :type "PrimitiveComponent Object Reference") (OtherActor :type "Actor Object Reference") (OtherComp :type "PrimitiveComponent Object Reference") (OtherBodyIndex :type Integer))
  (bind _returnvalue (`GameplayStatics.GetPlayerCharacter` 0))
  ;[1 1 1] Set Boolean on overlap and END overlap, active tick only on overlap to optimize
  (if (`self.ActorHasTag` OtherActor "Player")
    (set `self.Player in Area` false)
    (switch `string` (`self.Pick Damage Index (1+,1-,2+,2-)`)
      (:`1+`
        (bind _asbp_first_person_character (cast `/Game/LostBalance/Blueprints/Player/BP_FirstPersonCharacter` _returnvalue :!label _label_3))
        (`/Game/LostBalance/Blueprints/Player/BP_FirstPersonCharacter.Start Delay Bar 1` _asbp_first_person_character))
      (:`1-`
        (goto _label_3))
      (:`2+`
        (bind _asbp_first_person_character_2 (cast `/Game/LostBalance/Blueprints/Player/BP_FirstPersonCharacter` _returnvalue :!label _label_4))
        (`/Game/LostBalance/Blueprints/Player/BP_FirstPersonCharacter.Start Delay Bar 2` _asbp_first_person_character_2))
      (:`2-`
        (goto _label_4)))))

(fn `UserConstructionScript`)