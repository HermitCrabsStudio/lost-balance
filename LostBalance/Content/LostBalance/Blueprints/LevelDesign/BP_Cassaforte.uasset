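; BP_Cassaforte is an interactable safe in Lost Balance that the player unlocks through a UI screen.
; A trigger shows a widget component while a Player-tagged actor overlaps and the safe is still closed.
; Interact opens WBP_Cassaforte in UI-only input mode with a mouse cursor.
; ApriCassaforte removes that screen, marks the safe opened, restores game input and swings the door pivot open with a timeline.
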(event `self.Trigger.OnComponentBeginOverlap`
  (params (OverlappedComponent :type "PrimitiveComponent Object Reference") (OtherActor :type "Actor Object Reference") (OtherComp :type "PrimitiveComponent Object Reference") (OtherBodyIndex :type Integer) (bFromSweep :type Boolean) (SweepResult :type "HitResult Structure (by ref)"))
  (if (and (not (`self.Opened?`)) (`self.ActorHasTag` OtherActor "Player"))
    (`SceneComponent.SetVisibility` (`self.Widget`) true false)))

(event `self.Trigger.OnComponentEndOverlap`
  (params (OverlappedComponent :type "PrimitiveComponent Object Reference") (OtherActor :type "Actor Object Reference") (OtherComp :type "PrimitiveComponent Object Reference") (OtherBodyIndex :type Integer))
  (if (and (not (`self.Opened?`)) (`self.ActorHasTag` OtherActor "Player"))
    (`SceneComponent.SetVisibility` (`self.Widget`) false false)))

(event `/Game/LostBalance/Blueprints/Technical/BPI_Interaction.Interact`
  (bind _returnvalue (`GameplayStatics.GetPlayerController` 0))
  (bind _returnvalue_2 (`|CreateWidget` "/Game/LostBalance/UI/Widgets/WBP_Cassaforte.WBP_Cassaforte_C" _returnvalue))
  (`UserWidget.AddToViewport` _returnvalue_2 0)
  (set `self.ComputerAccesso` _returnvalue_2)
  (set `PlayerController.bShowMouseCursor` true _returnvalue)
  (`WidgetBlueprintLibrary.SetInputMode_UIOnlyEx` (`GameplayStatics.GetPlayerController` 0) _returnvalue_2))

(event `ApriCassaforte`
  (bind _returnvalue (`GameplayStatics.GetPlayerController` 0))
  (`Widget.RemoveFromParent` (`self.ComputerAccesso`))
  (set `self.Opened?` true)
  (`SceneComponent.SetVisibility` (`self.Widget`) false false)
  (`WidgetBlueprintLibrary.SetInputMode_GameOnly` _returnvalue)
  (set `PlayerController.bShowMouseCursor` false _returnvalue)
  (bind (_direction _open) (`Timeline|Open` :!via `PlayFromStart`)
    (:`Update`
      (`SceneComponent.K2_SetRelativeRotation` (`self.PivotPorta`) (`KismetMathLibrary.MakeRotator` 0.0 0.0 (`KismetMathLibrary.Lerp` 0.0 110.0 _open)) false false))))

(fn `UserConstructionScript`)