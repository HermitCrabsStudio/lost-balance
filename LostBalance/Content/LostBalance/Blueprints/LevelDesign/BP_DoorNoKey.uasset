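; BP_DoorNoKey is a door that opens without a key, once, when its Interact event is called.
; Left and right trigger volumes show or hide a prompt widget for their side as the Player-tagged actor overlaps them, until the door is opened.
; Interact sets DoorOpened, hides both widgets and plays a timeline that lerps the door's yaw to swing it open.
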(event `self.TriggerLeft.OnComponentBeginOverlap`
  (params (OverlappedComponent :type "PrimitiveComponent Object Reference") (OtherActor :type "Actor Object Reference") (OtherComp :type "PrimitiveComponent Object Reference") (OtherBodyIndex :type Integer) (bFromSweep :type Boolean) (SweepResult :type "HitResult Structure (by ref)"))
  ;[1 1 1] Set widgets visibility related to direction u come
  (if (`self.DoorOpened?`)
    _
    (elif (`self.ActorHasTag` OtherActor "Player")
      (`SceneComponent.SetVisibility` (`self.WidgetLeft`) true false))))

(event `self.TriggerLeft.OnComponentEndOverlap`
  (params (OverlappedComponent :type "PrimitiveComponent Object Reference") (OtherActor :type "Actor Object Reference") (OtherComp :type "PrimitiveComponent Object Reference") (OtherBodyIndex :type Integer))
  ;[1 1 1] Set widgets visibility related to direction u come
  (if (`self.DoorOpened?`)
    _
    (elif (`self.ActorHasTag` OtherActor "Player")
      (`SceneComponent.SetVisibility` (`self.WidgetLeft`) false false))))

(event `self.TriggerRight.OnComponentBeginOverlap`
  (params (OverlappedComponent :type "PrimitiveComponent Object Reference") (OtherActor :type "Actor Object Reference") (OtherComp :type "PrimitiveComponent Object Reference") (OtherBodyIndex :type Integer) (bFromSweep :type Boolean) (SweepResult :type "HitResult Structure (by ref)"))
  ;[1 1 1] Set widgets visibility related to direction u come
  (if (`self.DoorOpened?`)
    _
    (elif (`self.ActorHasTag` OtherActor "Player")
      (`SceneComponent.SetVisibility` (`self.WidgetRight`) true false))))

(event `self.TriggerRight.OnComponentEndOverlap`
  (params (OverlappedComponent :type "PrimitiveComponent Object Reference") (OtherActor :type "Actor Object Reference") (OtherComp :type "PrimitiveComponent Object Reference") (OtherBodyIndex :type Integer))
  ;[1 1 1] Set widgets visibility related to direction u come
  (if (`self.DoorOpened?`)
    _
    (elif (`self.ActorHasTag` OtherActor "Player")
      (`SceneComponent.SetVisibility` (`self.WidgetRight`) false false))))

(event `/Game/LostBalance/Blueprints/Technical/BPI_Interaction.Interact`
  ;[1 1 1] Player can open door only 1 time with the check, timeline make a lerp on door rotation to reach open position
  (if (not (`self.DoorOpened?`))
    (set `self.DoorOpened?` true)
    (`SceneComponent.SetVisibility` (`self.WidgetLeft`) false false)
    (`SceneComponent.SetVisibility` (`self.WidgetRight`) false false)
    (bind (_direction _dooropening) (`Timeline|DoorOpening` :!via `PlayFromStart`)
      (:`Update`
        (`SceneComponent.K2_SetRelativeRotation` (`self.DoorNoKey`) (`KismetMathLibrary.MakeRotator` 0.0 0.0 (`KismetMathLibrary.Lerp` 0.0 110.0 _dooropening)) false false)))))

(fn `UserConstructionScript`)