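; BP_Pistol is an interactable secret pickup placed in levels.
; ActivateInteraction enables the trigger's overlap events and arms the pickup, and the trigger shows or hides a prompt widget as the Player-tagged actor enters or leaves.
; When active, Interact displays a "secret found" tutorial message hinting at later story use, then destroys the actor without recording the pickup in this graph.
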(event `Activate Interaction`
  (set `PrimitiveComponent.bGenerateOverlapEvents` true (`self.Trigger`))
  (set `self.IsActive?` true))

(event `self.Trigger.OnComponentBeginOverlap`
  (params (OverlappedComponent :type "PrimitiveComponent Object Reference") (OtherActor :type "Actor Object Reference") (OtherComp :type "PrimitiveComponent Object Reference") (OtherBodyIndex :type Integer) (bFromSweep :type Boolean) (SweepResult :type "HitResult Structure (by ref)"))
  (if (`self.ActorHasTag` OtherActor "Player")
    (`SceneComponent.SetVisibility` (`self.Widget`) true false)))

(event `self.Trigger.OnComponentEndOverlap`
  (params (OverlappedComponent :type "PrimitiveComponent Object Reference") (OtherActor :type "Actor Object Reference") (OtherComp :type "PrimitiveComponent Object Reference") (OtherBodyIndex :type Integer))
  (if (`self.ActorHasTag` OtherActor "Player")
    (`SceneComponent.SetVisibility` (`self.Widget`) false false)))

(event `/Game/LostBalance/Blueprints/Technical/BPI_Interaction.Interact`
  (if (`self.IsActive?`)
    (bind _returnvalue (`|CreateWidget` "/Game/LostBalance/UI/Widgets/WBP_TextDialogueUpperScreen_Tutorial.WBP_TextDialogueUpperScreen_Tutorial_C" (`GameplayStatics.GetPlayerController` 0)))
    (`/Game/LostBalance/UI/Widgets/WBP_TextDialogueUpperScreen_Tutorial.Set Text Tutorial` _returnvalue "SECRET FOUND! SOME INTERACTION WILL REQUIRE IT LATER IN THE STORY" false)
    (`UserWidget.AddToViewport` _returnvalue 0)
    (`self.K2_DestroyActor`)))

(fn `UserConstructionScript`)