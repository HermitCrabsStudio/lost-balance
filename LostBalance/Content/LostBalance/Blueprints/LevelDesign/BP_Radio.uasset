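; BP_Radio is an interactable radio prop whose audio the player can switch off and on.
; Overlapping its trigger area with a Player-tagged actor shows a widget, hidden again on exit.
; Interact flip-flops the audio, stopping on the first call and restarting from the beginning on the next.
; A separate Distorcisuono event runs a timeline that modulates volume and pitch for distortion, flagging EffettoAudioON until it finishes.
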(event `self.TriggerArea.OnComponentBeginOverlap`
  (params (OverlappedComponent :type "PrimitiveComponent Object Reference") (OtherActor :type "Actor Object Reference") (OtherComp :type "PrimitiveComponent Object Reference") (OtherBodyIndex :type Integer) (bFromSweep :type Boolean) (SweepResult :type "HitResult Structure (by ref)"))
  (if (`self.ActorHasTag` OtherActor "Player")
    (`SceneComponent.SetVisibility` (`self.Widget`) true false)))

(event `self.TriggerArea.OnComponentEndOverlap`
  (params (OverlappedComponent :type "PrimitiveComponent Object Reference") (OtherActor :type "Actor Object Reference") (OtherComp :type "PrimitiveComponent Object Reference") (OtherBodyIndex :type Integer))
  (if (`self.ActorHasTag` OtherActor "Player")
    (`SceneComponent.SetVisibility` (`self.Widget`) false false)))

(event `/Game/LostBalance/Blueprints/Technical/BPI_Interaction.Interact`
  (bind _audio (`self.Audio`))
  (`/Engine/EditorBlueprintResources/StandardMacros.FlipFlop`
    (:`A`
      (`AudioComponent.Stop` _audio))
    (:`B`
      (`AudioComponent.Play` _audio 0.0))))

(event `Distorci suono`
  (bind _audio (`self.Audio`))
  ;[1 1 1] Distorci Suono
  (bind (_direction _distorci) (`Timeline|Timeline` :!via `PlayFromStart`)
    (:`Update`
      (set `self.EffettoAudioON` true)
      (`AudioComponent.SetVolumeMultiplier` _audio (`KismetMathLibrary.Lerp` 1.0 10.0 _distorci))
      (`AudioComponent.SetPitchMultiplier` _audio (`KismetMathLibrary.Lerp` 1.0 0.8 _distorci)))
    (:`Finished`
      (set `self.EffettoAudioON` false))))

(fn `UserConstructionScript`)