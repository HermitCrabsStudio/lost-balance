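; BP_Note_LootableVision is a lootable note placed in the level that the player picks up by interacting with it.
; Its trigger area shows a widget while an actor tagged Player overlaps it and hides the widget on exit.
; The Interact event passes the note's index to CallNoteWidget on BP_FirstPersonCharacter, then destroys the note actor.
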(event `self.Trigger Area.OnComponentBeginOverlap`
  (params (OverlappedComponent :type "PrimitiveComponent Object Reference") (OtherActor :type "Actor Object Reference") (OtherComp :type "PrimitiveComponent Object Reference") (OtherBodyIndex :type Integer) (bFromSweep :type Boolean) (SweepResult :type "HitResult Structure (by ref)"))
  ;[1 1 1] Set Widget Visibility
  (if (`self.ActorHasTag` OtherActor "Player")
    (`SceneComponent.SetVisibility` (`self.Widget`) true false)))

(event `self.Trigger Area.OnComponentEndOverlap`
  (params (OverlappedComponent :type "PrimitiveComponent Object Reference") (OtherActor :type "Actor Object Reference") (OtherComp :type "PrimitiveComponent Object Reference") (OtherBodyIndex :type Integer))
  ;[1 1 1] Set Widget Visibility
  (if (`self.ActorHasTag` OtherActor "Player")
    (`SceneComponent.SetVisibility` (`self.Widget`) false false)))

(event `self.Interact`
  ;[1 1 1] Event called on object interaction
  (bind _asbp_first_person_character (cast `/Game/LostBalance/Blueprints/Player/BP_FirstPersonCharacter` (`GameplayStatics.GetPlayerCharacter` 0)))
  (`/Game/LostBalance/Blueprints/Player/BP_FirstPersonCharacter.CallNoteWidget` _asbp_first_person_character (`self.SwitchIndexNote`))
  (`self.K2_DestroyActor`))

(fn `UserConstructionScript`)