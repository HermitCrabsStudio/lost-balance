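; BP_JukeBox is an interactable jukebox that the player can switch on and off to play a sound.
; A Sphere overlap shows the Widget while an actor tagged Player is in range and hides it on exit.
; Interact toggles IsActive, either spawning a new non-spatialized 2D sound at reduced volume and storing it in Audio, or deactivating that stored component.
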(event `self.Sphere.OnComponentBeginOverlap`
  (params (OverlappedComponent :type "PrimitiveComponent Object Reference") (OtherActor :type "Actor Object Reference") (OtherComp :type "PrimitiveComponent Object Reference") (OtherBodyIndex :type Integer) (bFromSweep :type Boolean) (SweepResult :type "HitResult Structure (by ref)"))
  ;[0.06366 1 0.6746] Widget Visibility
  (if (`self.ActorHasTag` OtherActor "Player")
    (`SceneComponent.SetVisibility` (`self.Widget`) true false)))

(event `self.Sphere.OnComponentEndOverlap`
  (params (OverlappedComponent :type "PrimitiveComponent Object Reference") (OtherActor :type "Actor Object Reference") (OtherComp :type "PrimitiveComponent Object Reference") (OtherBodyIndex :type Integer))
  ;[0.06366 1 0.6746] Widget Visibility
  (if (`self.ActorHasTag` OtherActor "Player")
    (`SceneComponent.SetVisibility` (`self.Widget`) false false)))

(event `/Game/LostBalance/Blueprints/Technical/BPI_Interaction.Interact`
  ;[0.1534 1 0.2165] Interaction Event
  (if (`self.isActive`)
    (`ActorComponent.SetActive` (`self.Audio`) false false)
    (set `self.isActive` false)
    (else
      (bind _returnvalue (`GameplayStatics.SpawnSound2D` "/Game/LostBalance/Assets/SFX/running-sounds-6003.running-sounds-6003" 0.25 1.0 0.0 null))
      (set `self.Audio` _returnvalue)
      (set `self.isActive` true))))

(fn `UserConstructionScript`)