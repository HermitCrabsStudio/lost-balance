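; Actor component that delays the restoration of bar 1 on the player's BP_FirstPersonCharacter by using its tick interval as a timer.
; Activate and deactivate events toggle ticking, with activation also setting the interval from DelayRestoreBar1 and resetting a counter.
; The first tick only advances the counter, then later ticks set the character's RestoreBar1Active flag if unset and print a debug message.
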(event `DeactivateRestoreDelayBar1`
  (`self.SetComponentTickEnabled` false))

(event `ActivateRestoreDelayBar1`
  (`self.SetComponentTickInterval` (`self.Delay Restore Bar 1`))
  (`self.SetComponentTickEnabled` true)
  (set `self.DebugIndex` 0))

(event `self.ReceiveBeginPlay`
  (`self.SetComponentTickInterval` (`self.Delay Restore Bar 1`)))

(event `self.ReceiveTick`
  (params (DeltaSeconds :type "Float (single-precision)"))
  ;[1 1 1] Delay the activation of the restorebar1 variable on character
  (switch `int` (`self.DebugIndex`)
    (:`0`
      (set `self.DebugIndex` 1))
    (:`1`
      (bind _asbp_first_person_character (cast `/Game/LostBalance/Blueprints/Player/BP_FirstPersonCharacter` (`GameplayStatics.GetPlayerCharacter` 0)))
      (if (not (`/Game/LostBalance/Blueprints/Player/BP_FirstPersonCharacter.RestoreBar1Active?` _asbp_first_person_character))
        (set `/Game/LostBalance/Blueprints/Player/BP_FirstPersonCharacter.RestoreBar1Active?` true _asbp_first_person_character)
        (`KismetSystemLibrary.PrintString` "RESTORE BAR 1 ACTIVATED" true true (struct :`G` 1.0 :`B` 0.339822 :`A` 1.0) 5.0)))))