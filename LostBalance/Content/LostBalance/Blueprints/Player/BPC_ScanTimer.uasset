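; Actor component that acts as a delay timer for de-scanning, calling DeScanAfterDelayDevice on the first-person player character.
; It uses its tick interval, set from DelayDeScan, as the countdown, with events to enable and disable ticking.
; An index reset on activation skips the immediate first tick, so the call lands on a later one.
; A DeScanDone flag keeps the call single-shot until deactivation resets it.
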(event `self.ReceiveBeginPlay`
  ;[1 1 1] Set tick interval on start
  (`self.SetComponentTickInterval` (`self.DelayDeScan`)))

(event `Active DeScan Delay`
  ;[1 1 1] Activate tick, set delay time and bug fixing index
  (`self.SetComponentTickInterval` (`self.DelayDeScan`))
  (`self.SetComponentTickEnabled` true)
  (set `self.IndexBugFixing` 0))

(event `Deactive DeScan Delay`
  ;[1 1 1] Deactivate tick - also reset bool for single shot function below
  (`self.SetComponentTickEnabled` false)
  (set `self.DeScanDone?` false))

(event `self.ReceiveTick`
  (params (DeltaSeconds :type "Float (single-precision)"))
  ;[1 1 1] Event tick (with switch for bug fixing, automatic call of tick event when enabled),
  (switch `int` (`self.IndexBugFixing`)
    (:`0`
      (set `self.IndexBugFixing` 1))
    (:`1`
      (bind _asbp_first_person_character (cast `/Game/LostBalance/Blueprints/Player/BP_FirstPersonCharacter` (`GameplayStatics.GetPlayerCharacter` 0)))
      (if (not (`self.DeScanDone?`))
        (set `self.DeScanDone?` true)
        (`/Game/LostBalance/Blueprints/Player/BP_FirstPersonCharacter.DeScan after delay (device)` _asbp_first_person_character)))))