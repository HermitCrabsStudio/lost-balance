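; Player stamina component that drains and restores stamina for the first-person character's sprint, using rates read from the character.
; EnableTick repurposes component tick as a timer, setting its interval and Consume or Restore mode, and skipping the first tick as a workaround.
; Empty stamina forces walking, blocks sprint and switches to Restore at a slower interval.
; Full stamina stops the tick and re-allows sprint.
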(event `Disable Tick`
  ;[1 1 1] Deactivate tick after (called on descan)
  (`self.SetComponentTickEnabled` false))

(event `Enable Tick`
  (params (DelayFunction :type "Float (double-precision)") (FunctionName :type String))
  ;[1 1 1] Activate tick, set tick delay and set switch index for bug fixing
  (`self.SetComponentTickInterval` DelayFunction)
  (`self.SetComponentTickEnabled` false)
  (`self.SetComponentTickEnabled` true)
  (set `self.DebugIndex` 0)
  (set `self.FunctionIndex` FunctionName))

(event `self.ReceiveBeginPlay`
  ;[1 1 1] On begin play set descan delay
  (`self.SetComponentTickInterval` 0.0)
  (bind _asbp_first_person_character (cast `/Game/LostBalance/Blueprints/Player/BP_FirstPersonCharacter` (`GameplayStatics.GetPlayerCharacter` 0)))
  (set `self.StaminaConsumeValue` (`/Game/LostBalance/Blueprints/Player/BP_FirstPersonCharacter.Stamina consume Value` _asbp_first_person_character))
  (set `self.StaminaRestoreValue` (`/Game/LostBalance/Blueprints/Player/BP_FirstPersonCharacter.Stamina restore Value` _asbp_first_person_character)))

(event `self.ReceiveTick`
  (params (DeltaSeconds :type "Float (single-precision)"))
  ;[1 1 1] Delay the activation of the restorebar1 variable on character
  (switch `int` (`self.DebugIndex`)
    (:`0`
      (set `self.DebugIndex` 1)
      (`KismetSystemLibrary.PrintString` "tick  debug"))
    (:`1`
      (switch `string` (`self.FunctionIndex`)
        (:`Default`
          (`KismetSystemLibrary.PrintString` "DEFAULT"))
        (:`Consume`
          (if (> (`self.Stamina`) 0.0)
            (set `self.Stamina` (- (`self.Stamina`) (`self.StaminaConsumeValue`)))
            (else
              (set `self.Stamina` 0.0)
              (bind _asbp_first_person_character (cast `/Game/LostBalance/Blueprints/Player/BP_FirstPersonCharacter` (`GameplayStatics.GetPlayerCharacter` 0)))
              (`/Game/LostBalance/Blueprints/Player/BP_FirstPersonCharacter.Call Walk` _asbp_first_person_character)
              (set `/Game/LostBalance/Blueprints/Player/BP_FirstPersonCharacter.CanSprint?` false _asbp_first_person_character)
              (`KismetSystemLibrary.PrintString` "STAMINA FINISHED")
              (`self.Enable Tick` 5.0 "Restore")
              (`KismetSystemLibrary.PrintString` "CALLED RESPAWN"))))
        (:`Restore`
          (if (< (`self.Stamina`) 100.0)
            (set `self.Stamina` (+ (`self.Stamina`) (`self.StaminaRestoreValue`)))
            (`KismetSystemLibrary.PrintString` "RESTORING")
            (else
              (set `self.Stamina` 100.0)
              (`self.Disable Tick`)
              (`KismetSystemLibrary.PrintString` "STAMINA MAX")
              (bind _asbp_first_person_character_2 (cast `/Game/LostBalance/Blueprints/Player/BP_FirstPersonCharacter` (`GameplayStatics.GetPlayerCharacter` 0)))
              (set `/Game/LostBalance/Blueprints/Player/BP_FirstPersonCharacter.CanSprint?` true _asbp_first_person_character_2))))))))