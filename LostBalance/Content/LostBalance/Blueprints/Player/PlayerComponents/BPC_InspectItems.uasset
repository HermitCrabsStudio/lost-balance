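; BPC_InspectItems is a player component that rotates the model of an item being inspected.
; Each Tick it casts player 0's character to BP_FirstPersonCharacter and checks its RotatingModelZ and RotatingModelX flags.
; Active flags add local yaw or roll to InspectItemModel, scaling RotationAngle by delta time for frame-rate-independent spin, and both axes can turn at once.
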(event `self.ReceiveTick`
  (params (DeltaSeconds :type "Float (single-precision)"))
  (bind _asbp_first_person_character (cast `/Game/LostBalance/Blueprints/Player/BP_FirstPersonCharacter` (`GameplayStatics.GetPlayerCharacter` 0)))
  (`|ExecutionSequence`
    (:`then_0`
      (if (`/Game/LostBalance/Blueprints/Player/BP_FirstPersonCharacter.rotatingModel Z` _asbp_first_person_character)
        (`SceneComponent.K2_AddLocalRotation` (`/Game/LostBalance/Blueprints/Player/BP_FirstPersonCharacter.Inspect Item Model` _asbp_first_person_character) (`KismetMathLibrary.MakeRotator` 0.0 0.0 (* DeltaSeconds (`self.Rotation Angle`))) false false)))
    (:`then_1`
      (if (`/Game/LostBalance/Blueprints/Player/BP_FirstPersonCharacter.rotatingModel X` _asbp_first_person_character)
        (`SceneComponent.K2_AddLocalRotation` (`/Game/LostBalance/Blueprints/Player/BP_FirstPersonCharacter.Inspect Item Model` _asbp_first_person_character) (`KismetMathLibrary.MakeRotator` (* DeltaSeconds (`self.Rotation Angle`))) false false)))))