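; Player component that delays setting RestoreBar1Active on the first-person character, using its own tick interval as the timer.
; ActivateRestoreDelayBar1 enables tick at the DelayRestoreBar1 interval and resets DebugIndex, which makes the first tick a no-op as a bug workaround.
; Later ticks set the character flag if it is not already set.
; DeactivateRestoreDelayBar1, noted as called on descan, disables tick and clears CanRestore, which only gates debug prints here.
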(event `DeactivateRestoreDelayBar1`
  ;[1 1 1] Deactivate tick after (called on descan)
  (`self.SetComponentTickEnabled` false)
  (if (`self.CanRestore?`)
    (bind _output_get (set `self.CanRestore?` false))
    (`KismetSystemLibrary.PrintString` "Hello" _output_get)))

(event `ActivateRestoreDelayBar1`
  ;[1 1 1] Activate tick, set tick delay and set switch index for bug fixing
  (`self.SetComponentTickInterval` (`self.Delay Restore Bar 1`))
  (`self.SetComponentTickEnabled` true)
  (set `self.DebugIndex` 0)
  (if (not (`self.CanRestore?`))
    (bind _output_get (set `self.CanRestore?` true))
    (`KismetSystemLibrary.PrintString` (`KismetStringLibrary.Conv_BoolToString` _output_get))))

(event `self.ReceiveBeginPlay`
  ;[1 1 1] On begin play set descan delay
  (`self.SetComponentTickInterval` (`self.Delay Restore Bar 1`)))

(event `self.ReceiveTick`
  (params (DeltaSeconds :type "Float (single-precision)"))
  ;[1 1 1] Delay the activation of the restorebar1 variable on character
  (switch `int` (`self.DebugIndex`)
    (:`0`
      (set `self.DebugIndex` 1))
    (:`1`
      (bind _asbp_first_person_character (cast `/Game/LostBalance/Blueprints/Player/BP_FirstPersonCharacter` (`GameplayStatics.GetPlayerCharacter` 0)))
      (if (not (`/Game/LostBalance/Blueprints/Player/BP_FirstPersonCharacter.RestoreBar1Active?` _asbp_first_person_character))
        (set `/Game/LostBalance/Blueprints/Player/BP_FirstPersonCharacter.RestoreBar1Active?` true _asbp_first_person_character)))))