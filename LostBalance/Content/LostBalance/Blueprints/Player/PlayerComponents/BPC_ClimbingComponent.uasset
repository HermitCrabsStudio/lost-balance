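; BPC_ClimbingComponent is a player component that detects and drives climbing for BP_FirstPersonCharacter.
; ActiveRayCast enables its tick, while DeactiveRayCast disables it and resets the state index.
; Tick runs a two-state switch: the first calls the character's climbing line trace, then either triggers ClimbingCall and advances on a hit or deactivates on a miss.
; The second state calls the character's ClimbingLoop every tick until deactivated.
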(event `Deactive RayCast`
  (`self.SetComponentTickEnabled` false)
  (set `self.TestIndex` 0)
  (`KismetSystemLibrary.PrintString` "called deactive"))

(event `Active RayCast`
  (`self.SetComponentTickEnabled` true)
  (`KismetSystemLibrary.PrintString` "called active"))

(event `self.ReceiveTick`
  (params (DeltaSeconds :type "Float (single-precision)"))
  (switch `int` (`self.TestIndex`)
    (:`0`
      (bind _asbp_first_person_character (cast `/Game/LostBalance/Blueprints/Player/BP_FirstPersonCharacter` (`GameplayStatics.GetPlayerCharacter` 0))
        (:`then`
          (bind (_hit_result _has_hit) (`/Game/LostBalance/Blueprints/Player/BP_FirstPersonCharacter.Climbing Line Trace` _asbp_first_person_character))
          (if _has_hit
            (`/Game/LostBalance/Blueprints/Player/BP_FirstPersonCharacter.Climbing Call` _asbp_first_person_character)
            (set `self.TestIndex` 1)
            (else
              (`self.Deactive RayCast`))))
        (:`CastFailed`
          (`KismetSystemLibrary.PrintString` "CAST FAILED"))))
    (:`1`
      (bind _asbp_first_person_character_2 (cast `/Game/LostBalance/Blueprints/Player/BP_FirstPersonCharacter` (`GameplayStatics.GetPlayerCharacter` 0)))
      (`/Game/LostBalance/Blueprints/Player/BP_FirstPersonCharacter.Climbing Loop` _asbp_first_person_character_2))))