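; Player component that delays restoration of the second bar on BP_FirstPersonCharacter.
; It uses its tick interval, set from DelayRestoreBar2, as a timer, with activate and deactivate events toggling tick and the CanRestore flag.
; DebugIndex makes the first tick after activation a skip, so later ticks set the character's RestoreBar2Active flag.
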(event `DeactivateRestoreDelayBar2`
  (`self.SetComponentTickEnabled` false)
  (if (`self.CanRestore?`)
    (set `self.CanRestore?` false)))

(event `ActivateRestoreDelayBar2`
  (`self.SetComponentTickInterval` (`self.Delay Restore Bar 2`))
  (`self.SetComponentTickEnabled` true)
  (set `self.Debug Index` 0)
  (if (not (`self.CanRestore?`))
    (set `self.CanRestore?` true)))

(event `self.ReceiveBeginPlay`
  (`self.SetComponentTickInterval` (`self.Delay Restore Bar 2`)))

(event `self.ReceiveTick`
  (params (DeltaSeconds :type "Float (single-precision)"))
  ;[1 1 1] Delay the activation of the restorebar1 variable on character
  (switch `int` (`self.Debug Index`)
    (:`0`
      (set `self.Debug Index` 1))
    (:`1`
      (bind _asbp_first_person_character (cast `/Game/LostBalance/Blueprints/Player/BP_FirstPersonCharacter` (`GameplayStatics.GetPlayerCharacter` 0)))
      (if (not (`/Game/LostBalance/Blueprints/Player/BP_FirstPersonCharacter.RestoreBar2Active?` _asbp_first_person_character))
        (set `/Game/LostBalance/Blueprints/Player/BP_FirstPersonCharacter.RestoreBar2Active?` true _asbp_first_person_character)))))