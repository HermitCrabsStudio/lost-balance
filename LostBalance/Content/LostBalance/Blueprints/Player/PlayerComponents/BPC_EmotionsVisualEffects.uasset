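; Player component that drives the visual effects for anxiety, fear and calm from the first-person character's emotion values.
; Each Tick it compares two emotion values against thresholds and calls the matching character effect, or its reverse when that emotion's NeedReverse flag is set.
; All three forward effects, calm included, also trigger a hard-breathing 2D sound, gated by a flag and delay to avoid overlapping playback.
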(event `self.ReceiveBeginPlay`
  (bind _asbp_first_person_character (cast `/Game/LostBalance/Blueprints/Player/BP_FirstPersonCharacter` (`GameplayStatics.GetPlayerCharacter` 0)))
  (set `self.As BP First Person Character` _asbp_first_person_character))

(event `self.ReceiveTick`
  (params (DeltaSeconds :type "Float (single-precision)"))
  (bind _as_bp_first_person_character (`self.As BP First Person Character`))
  (bind _as_bp_first_person_character_2 (`self.As BP First Person Character`))
  (bind _as_bp_first_person_character_3 (`self.As BP First Person Character`))
  (bind _emozione_1_copia (`/Game/LostBalance/Blueprints/Player/BP_FirstPersonCharacter.Emozione 1 Copia` _as_bp_first_person_character))
  ;[1 1 1] CALL EFFECT AND REVERSE IF VALUE GO OVER/UNDER THE LIMIT
  (`|ExecutionSequence`
    (:`then_0`
      (if (< _emozione_1_copia -50.0)
        (if (not (`self.NeedReverseAnx?`))
          (`/Game/LostBalance/Blueprints/Player/BP_FirstPersonCharacter.EFFETTO ANSIA` _as_bp_first_person_character_3)
          (`self.Player Effect Sound` :!label _label)
          (else
            (`/Game/LostBalance/Blueprints/Player/BP_FirstPersonCharacter.Reverse Anxiety effect` _as_bp_first_person_character_3)))))
    (:`then_1`
      (if (< (`/Game/LostBalance/Blueprints/Player/BP_FirstPersonCharacter.Emozione 2 Copia` _as_bp_first_person_character) -50.0)
        (if (not (`self.NeedReverseFear?`))
          (`/Game/LostBalance/Blueprints/Player/BP_FirstPersonCharacter.EFFETTO FEAR` _as_bp_first_person_character_3)
          (goto _label)
          (else
            (`/Game/LostBalance/Blueprints/Player/BP_FirstPersonCharacter.Reverse Fear Effect` _as_bp_first_person_character_3)))))
    (:`then_2`
      (if (> _emozione_1_copia 50.0)
        (if (not (`self.NeedReverseCalm?`))
          (`/Game/LostBalance/Blueprints/Player/BP_FirstPersonCharacter.EFFETTO CALMA` _as_bp_first_person_character_2)
          (goto _label)
          (else
            (`/Game/LostBalance/Blueprints/Player/BP_FirstPersonCharacter.Revers calm effect` _as_bp_first_person_character_2)))))))

(event `Player Effect Sound`
  (if (not (`self.isPlayingSound?`))
    (set `self.isPlayingSound?` true)
    (`GameplayStatics.PlaySound2D` "/Game/LostBalance/MusicSound/sound-effect-breathing-hard-122341.sound-effect-breathing-hard-122341" 1.0 1.0 0.0 null null)
    (`KismetSystemLibrary.Delay` 13.4)
    (set `self.isPlayingSound?` false)))