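; Pickup actor for the Emodex prototype emotion-scanning device, which the player collects by interacting with it.
; A trigger area shows or hides a widget as the player enters or leaves it.
; Interacting flags the first-person character as owning and equipping the device, reveals its device mesh, saves that state and toggles the device hint.
; It then displays a timed on-screen control hint and destroys itself.
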(event `/Game/LostBalance/Blueprints/Technical/BPI_Interaction.Interact`
  ;[1 1 1] Cast the device to the player (simply set boolean for prot and make the static mesh visible)
  (bind _asbp_first_person_character (cast `/Game/LostBalance/Blueprints/Player/BP_FirstPersonCharacter` (`GameplayStatics.GetPlayerCharacter` 0)))
  (set `/Game/LostBalance/Blueprints/Player/BP_FirstPersonCharacter.GotDevice?` true _asbp_first_person_character)
  (`SceneComponent.SetHiddenInGame` (`/Game/LostBalance/Blueprints/Player/BP_FirstPersonCharacter.DeviceMesh` _asbp_first_person_character) false false)
  (set `/Game/LostBalance/Blueprints/Player/BP_FirstPersonCharacter.DeviceEquipped?` true _asbp_first_person_character)
  (`/Game/LostBalance/Blueprints/Player/BP_FirstPersonCharacter.SaveDevice` _asbp_first_person_character)
  (`/Game/LostBalance/Blueprints/Player/BP_FirstPersonCharacter.Toggle Device Hint` _asbp_first_person_character)
  (bind _returnvalue (`|CreateWidget` "/Game/LostBalance/UI/Widgets/WBP_TextDialogueUpperScreen.WBP_TextDialogueUpperScreen_C" (`GameplayStatics.GetPlayerController` 0)))
  (`/Game/LostBalance/UI/Widgets/WBP_TextDialogueUpperScreen.Set TextandDelayfadeout` _returnvalue "Press Q to scan the emotions around \nPress X to toggle equip" 5.0 false)
  (`UserWidget.AddToViewport` _returnvalue 0)
  (`self.K2_DestroyActor`))

(event `self.TriggerArea.OnComponentBeginOverlap`
  (params (OverlappedComponent :type "PrimitiveComponent Object Reference") (OtherActor :type "Actor Object Reference") (OtherComp :type "PrimitiveComponent Object Reference") (OtherBodyIndex :type Integer) (bFromSweep :type Boolean) (SweepResult :type "HitResult Structure (by ref)"))
  (if (`self.ActorHasTag` OtherActor "Player")
    (`SceneComponent.SetHiddenInGame` (`self.Widget`) false false)))

(event `self.TriggerArea.OnComponentEndOverlap`
  (params (OverlappedComponent :type "PrimitiveComponent Object Reference") (OtherActor :type "Actor Object Reference") (OtherComp :type "PrimitiveComponent Object Reference") (OtherBodyIndex :type Integer))
  (if (`self.ActorHasTag` OtherActor "Player")
    (`SceneComponent.SetHiddenInGame` (`self.Widget`) true false)))

(fn `UserConstructionScript`)