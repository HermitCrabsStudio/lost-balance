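; BP_TriggerEmozione2 is a trigger volume that deals emotional damage to the player while they stay inside it.
; Begin and end overlaps on TriggerEmozione set the PlayerInArea flag for actors tagged Player.
; While the flag is set, Tick, noted as running once per second, adds DamageEmotivo to the first-person character's Emozione1Copia, despite the asset's "2" suffix.
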(event `self.ReceiveTick`
  (params (DeltaSeconds :type "Float (single-precision)"))
  ;[1 1 1] Tick any x seconds (1 actually) and cause emotional damage to BP_FirstPersonCharacter, CHECK BOOLEAN
  (if (`self.PlayerInArea?`)
    (bind _asbp_first_person_character (cast `/Game/FirstPerson/Blueprints/BP_FirstPersonCharacter` (`GameplayStatics.GetPlayerCharacter` 0)))
    (set `/Game/FirstPerson/Blueprints/BP_FirstPersonCharacter.Emozione 1 Copia` (+ (`/Game/FirstPerson/Blueprints/BP_FirstPersonCharacter.Emozione 1 Copia` _asbp_first_person_character) (`self.DamageEmotivo`)) _asbp_first_person_character)))

(event `self.TriggerEmozione.OnComponentBeginOverlap`
  (params (OverlappedComponent :type "PrimitiveComponent Object Reference") (OtherActor :type "Actor Object Reference") (OtherComp :type "PrimitiveComponent Object Reference") (OtherBodyIndex :type Integer) (bFromSweep :type Boolean) (SweepResult :type "HitResult Structure (by ref)"))
  ;[1 1 1] Set Boolean on overlap and END overlap
  (if (`self.ActorHasTag` OtherActor "Player")
    (set `self.PlayerInArea?` true)))

(event `self.TriggerEmozione.OnComponentEndOverlap`
  (params (OverlappedComponent :type "PrimitiveComponent Object Reference") (OtherActor :type "Actor Object Reference") (OtherComp :type "PrimitiveComponent Object Reference") (OtherBodyIndex :type Integer))
  ;[1 1 1] Set Boolean on overlap and END overlap
  (if (`self.ActorHasTag` OtherActor "Player")
    (set `self.PlayerInArea?` false)))

(fn `UserConstructionScript`)