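; BP_TriggerShaderEffect is a trigger volume that turns a post-process material effect on while the player is inside it.
; It finds the PostProcessController at BeginPlay and shows the material's name on a TextRender.
; Player overlap passes the material to the controller at full weight through a DoOnce.
; Any actor leaving resets the DoOnce and sets the weight to zero, with no Player tag check.
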(event `self.ReceiveBeginPlay`
  (bind _returnvalue (`GameplayStatics.GetActorOfClass` "/Game/LostBalance/Blueprints/Volumes/PostProcessController.PostProcessController_C"))
  (set `self.PostProcessController` _returnvalue)
  (`TextRenderComponent.K2_SetText` (`self.TextRender`) (`KismetTextLibrary.Conv_StringToText` (`KismetSystemLibrary.GetDisplayName` (`self.PPMaterial`)))))

(event `self.ReceiveActorBeginOverlap`
  (params (OtherActor :type "Actor Object Reference"))
  (if (`self.ActorHasTag` OtherActor "Player")
    (`/Engine/EditorBlueprintResources/StandardMacros.DoOnce` false :!label _label
      (:`Completed`
        (`/Game/LostBalance/Blueprints/Volumes/PostProcessController.ChangeMaterial` (`self.PostProcessController`) 0 1.0 (`self.PPMaterial`))))))

(event `self.ReceiveActorEndOverlap`
  (params (OtherActor :type "Actor Object Reference"))
  (`|ExecutionSequence`
    (:`then_0`
      (goto _label :!via `Reset`))
    (:`then_1`
      (`/Game/LostBalance/Blueprints/Volumes/PostProcessController.ChangeMaterial` (`self.PostProcessController`) 0 0.0 (`self.PPMaterial`)))))

(fn `UserConstructionScript`)