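; PPController actor that toggles a test post-process material in response to the first-person character's Emozione1 value.
; BeginPlay caches the player and the PostProcessVolume returned by a class lookup.
; Tick compares Emozione1Copia to a threshold, using paired Gates and DoOnces so changes fire only on crossings.
; ChangeMaterial writes PPM_TestPostProcess into the volume's material array at full or zero weight.
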(event `self.ReceiveBeginPlay`
  (bind _returnvalue (`GameplayStatics.GetActorOfClass` "/Script/Engine.PostProcessVolume"))
  (`/Engine/EditorBlueprintResources/StandardMacros.IsValid` _returnvalue
    (:`Is Valid`
      (set `self.PostProcess` _returnvalue)
      (set `self.Player` (`GameplayStatics.GetPlayerCharacter` 0)))
    (:`Is Not Valid`
      (`KismetSystemLibrary.PrintString` "PPController: PPVolume not found"))))

(event `self.ReceiveTick`
  (params (DeltaSeconds :type "Float (single-precision)"))
  (bind _asbp_first_person_character (cast `/Game/FirstPerson/Blueprints/BP_FirstPersonCharacter` (`self.Player`)))
  (bind _output_get (set `self.bPPEmozione1` (>= (`/Game/FirstPerson/Blueprints/BP_FirstPersonCharacter.Emozione 1 Copia` _asbp_first_person_character) (`self.Emozione1PPValue`))))
  (if _output_get
    (`|ExecutionSequence`
      (:`then_0`
        (goto _label :!via `Open`))
      (:`then_1`
        (`/Engine/EditorBlueprintResources/StandardMacros.Gate` true :!label _label
          (:`Exit`
            (`/Engine/EditorBlueprintResources/StandardMacros.DoOnce` false :!label _label_2
              (:`Completed`
                (`self.ChangeMaterial` 0 1.0))))))
      (:`then_2`
        (goto _label_3 :!via `Close`))
      (:`then_3`
        (goto _label_4 :!via `Reset`)))
    (else
      (`|ExecutionSequence`
        (:`then_0`
          (goto _label :!via `Close`))
        (:`then_1`
          (goto _label_2 :!via `Reset`))
        (:`then_2`
          (goto _label_3 :!via `Open`))
        (:`then_3`
          (`/Engine/EditorBlueprintResources/StandardMacros.Gate` true :!label _label_3
            (:`Exit`
              (`/Engine/EditorBlueprintResources/StandardMacros.DoOnce` false :!label _label_4
                (:`Completed`
                  (`self.ChangeMaterial` 0))))))))))

(event `ChangeMaterial`
  (params (MaterialIndex :type Integer) (Weight :type "Float (double-precision)"))
  (bind _weightedblendables_array (break `WeightedBlendables` (break `PostProcessSettings` (`PostProcessVolume.Settings` (`self.PostProcess`)))))
  (`KismetArrayLibrary.Array_Set` _weightedblendables_array MaterialIndex (make `WeightedBlendable` Weight "/Game/LostBalance/Materials/Shaders/PPM_TestPostProcess.PPM_TestPostProcess"))
  (`KismetSystemLibrary.PrintString` "PPController: Settings changed"))

(fn `UserConstructionScript`)