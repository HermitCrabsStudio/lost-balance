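; Toxic gas area that shifts one of the player's two emotion values while they stand inside its trigger.
; Overlap events for actors tagged Player set an in-area flag and toggle actor tick, whose configurable interval is applied at BeginPlay.
; Each tick, DamageFunction casts to BP_FirstPersonCharacter and uses a string selector to add or subtract the damage amount on the chosen emotion axis.
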(event `self.ReceiveBeginPlay`
  ;[1 1 1] You can set tick interval from inspector, will be setted up at the begin play
  (`self.SetActorTickInterval` (`self.Tick Interval Value`)))

(event `self.ReceiveTick`
  (params (DeltaSeconds :type "Float (single-precision)"))
  ;[1 1 1] Call Damage function when tick enabled
  (`self.Damage Function`))

(event `self.ToxicTriggef.OnComponentBeginOverlap`
  (params (OverlappedComponent :type "PrimitiveComponent Object Reference") (OtherActor :type "Actor Object Reference") (OtherComp :type "PrimitiveComponent Object Reference") (OtherBodyIndex :type Integer) (bFromSweep :type Boolean) (SweepResult :type "HitResult Structure (by ref)"))
  ;[1 1 1] Enable/Disable tick and set boolean for tick function
  (if (`self.ActorHasTag` OtherActor "Player")
    (set `self.Player In Area?` true)
    (`self.SetActorTickEnabled` true)))

(event `self.ToxicTriggef.OnComponentEndOverlap`
  (params (OverlappedComponent :type "PrimitiveComponent Object Reference") (OtherActor :type "Actor Object Reference") (OtherComp :type "PrimitiveComponent Object Reference") (OtherBodyIndex :type Integer))
  ;[1 1 1] Enable/Disable tick and set boolean for tick function
  (if (`self.ActorHasTag` OtherActor "Player")
    (set `self.Player In Area?` false)
    (`self.SetActorTickEnabled` false)))

(fn `Damage Function`
  (bind _value_damage_emotivo (`self.Value Damage Emotivo`))
  ;[1 1 1] Check boolean and cast to player
  (if (`self.Player In Area?`)
    (bind _asbp_first_person_character (cast `/Game/FirstPerson/Blueprints/BP_FirstPersonCharacter` (`GameplayStatics.GetPlayerCharacter` 0)))
    ;[1 1 1] Based on the string, switch the "side" of damage on the two axes (1+,1-,2+,2-)
    (switch `string` (`self.Pick Damage Side (1+,1-,2+,2-)`)
      (:`Default`
        (`KismetSystemLibrary.PrintString` "ERROR ON GAS TOXIC SWITCH "))
      (:`1+`
        (bind _emozione_1_copia (`/Game/FirstPerson/Blueprints/BP_FirstPersonCharacter.Emozione 1 Copia` _asbp_first_person_character))
        (set `/Game/FirstPerson/Blueprints/BP_FirstPersonCharacter.Emozione 1 Copia` (+ _emozione_1_copia _value_damage_emotivo) _asbp_first_person_character))
      (:`1-`
        (set `/Game/FirstPerson/Blueprints/BP_FirstPersonCharacter.Emozione 1 Copia` (- _emozione_1_copia _value_damage_emotivo) _asbp_first_person_character))
      (:`2+`
        (bind _emozione_2_copia (`/Game/FirstPerson/Blueprints/BP_FirstPersonCharacter.Emozione 2 Copia` _asbp_first_person_character))
        (set `/Game/FirstPerson/Blueprints/BP_FirstPersonCharacter.Emozione 2 Copia` (+ _emozione_2_copia _value_damage_emotivo) _asbp_first_person_character))
      (:`2-`
        (set `/Game/FirstPerson/Blueprints/BP_FirstPersonCharacter.Emozione 2 Copia` (- _emozione_2_copia _value_damage_emotivo) _asbp_first_person_character)))))

(fn `UserConstructionScript`)